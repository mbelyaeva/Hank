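; Hank is a player-controlled character that interacts with household objects and tracks a suspicion level that flags game over at its cap.
; The Interact input uses InteractionArea overlaps to trigger the breaker or light switch, grab or drop holdables, or destroy webs while holding something.
; Specific objects are checked by reference, with closest-target selection still marked TODO.
; Tick bobs the sprite on a real-time sine wave and highlights the Duster when grabbable.
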(event `InputAction|Interact`
  (params (Key :type "Key Structure" :default "AnyKey"))
  (bind _overlappingactors (`PrimitiveComponent.GetOverlappingActors` (`self.InteractionArea`) null))
  (bind _overlappingactors_2 (`PrimitiveComponent.GetOverlappingActors` (`self.InteractionArea`) null))
  (bind _overlappingactors_3 (`PrimitiveComponent.GetOverlappingActors` (`self.InteractionArea`) "/Game/Hank/Blueprints/HoldableObject.HoldableObject_C"))
  (:`Pressed`
    (if (and (not (`KismetArrayLibrary.Array_Contains` _overlappingactors_2 (`self.web1`))) (not (`KismetArrayLibrary.Array_Contains` _overlappingactors_2 (`self.web2`))) (`KismetArrayLibrary.Array_Contains` _overlappingactors_2 (`self.breaker`)))
      (`/Game/Hank/Blueprints/InteractableObject.Interaction` (`self.breaker`))
      (elif (`self.holding`)
        (if (`KismetArrayLibrary.Array_Contains` _overlappingactors (`self.web2`))
          (if (`KismetArrayLibrary.Array_Contains` _overlappingactors (`self.web1`))
            (`self.K2_DestroyActor` (`self.web1`))
            (else
              (`self.K2_DestroyActor` (`self.web2`))))
          (else
            ;[1 1 1] Drop held item
            (`/Game/Hank/Blueprints/HoldableObject.Event Dropped` (`self.heldObject`))
            (set `self.holding` false)))
        (else
          ;[1 1 1] Pick up item if in range
          (if (> (`KismetArrayLibrary.Array_Length` _overlappingactors_3) 0)
            (bind _asholdable_object (cast `/Game/Hank/Blueprints/HoldableObject` (`KismetArrayLibrary.Array_Get` _overlappingactors_3)))
            (if (`/Game/Hank/Blueprints/HoldableObject.held` _asholdable_object)
              ;[1 1 1] Hit lightswitch if in range
              (if (`KismetArrayLibrary.Array_Contains` (`PrimitiveComponent.GetOverlappingActors` (`self.InteractionArea`) "/Game/Hank/Blueprints/InteractableObject.InteractableObject_C") (`self.lightswitch`)) :!label _label
                (`/Game/Hank/Blueprints/InteractableObject.Interaction` (`self.lightswitch`)))
              (else
                (`/Game/Hank/Blueprints/HoldableObject.Event GrabbedByHank` _asholdable_object)
                (set `self.heldObject` _asholdable_object)
                (set `self.holding` true)))
            (else
              (goto _label))))))))

(event `self.ReceiveTick`
  (params (DeltaSeconds :type "Float (single-precision)"))
  (bind (_seconds _partialseconds) (`GameplayStatics.GetAccurateRealTime`))
  (bind _duster (`self.duster`))
  (`SceneComponent.K2_SetRelativeLocation` (`self.Sprite`) (`KismetMathLibrary.MakeVector` 0.0 0.0 (* (`KismetMathLibrary.DegSin` (* (+ (`KismetMathLibrary.Conv_IntToDouble` (mod _seconds 360)) _partialseconds) 200.0)) 5.0)) false false)
  (if (`KismetSystemLibrary.IsValid` (`self.duster`))
    (`SceneComponent.SetVisibility` (`/Game/Hank/Blueprints/HoldableObject.Highlight` _duster) (and (`KismetArrayLibrary.Array_Contains` (`PrimitiveComponent.GetOverlappingActors` (`self.InteractionArea`) "/Game/Hank/Blueprints/HoldableObject.HoldableObject_C") _duster) (not (`/Game/Hank/Blueprints/HoldableObject.held` _duster))) false)))

(fn `addSuspicion`
  (params (`Suspicion increase` :type "Float (double-precision)"))
  (bind _output_get (set `self.suspicion` (`KismetMathLibrary.FMin` (+ `Suspicion increase` (`self.suspicion`)) 100.0)))
  (if (== _output_get 100.0)
    (set `self.gameOver` true)))

(fn `getSuspicion`
  (returns (Suspicion :type "Float (double-precision)"))
  (return (`self.suspicion`)))

(fn `UserConstructionScript`)