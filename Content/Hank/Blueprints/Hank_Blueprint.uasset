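; Hank_Blueprint uses number keys 1 to 5 to fire scripted events on scene objects, apparently a scare sequence.
; The keys turn the lights off, trigger the duster's grab event, destroy two webs, swap the breaker for an open version, and kill the lights while triggering Grandma's scare-out.
; The breaker swap spawns Breakers_Open at the destroyed actor's saved transform.
; All other graphs are empty.
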(event `self.ReceiveBeginPlay`)

(event `InputAction|Interact`
  (params (Key :type "Key Structure" :default "AnyKey")))

(event `Key|One`
  (params (Key :type "Key Structure" :default "AnyKey"))
  (:`Pressed`
    (`/Game/Hank/Blueprints/Lightswitch.Event LightsOff` (`self.lightswitch`))))

(event `self.ReceiveActorBeginOverlap`
  (params (OtherActor :type "Actor Object Reference")))

(event `Key|Two`
  (params (Key :type "Key Structure" :default "AnyKey"))
  (:`Pressed`
    (`/Game/Hank/Blueprints/Duster.Event Grabbed` (`self.duster`))))

(event `self.ReceiveTick`
  (params (DeltaSeconds :type "Float (single-precision)")))

(event `Key|Three`
  (params (Key :type "Key Structure" :default "AnyKey"))
  (:`Pressed`
    (`self.K2_DestroyActor` (`self.web1`))
    (`self.K2_DestroyActor` (`self.web2`))))

(event `Key|Four`
  (params (Key :type "Key Structure" :default "AnyKey"))
  (:`Pressed`
    (set `self.breakertrans` (`self.GetTransform` (`self.breaker`)))
    (`self.K2_DestroyActor` (`self.breaker`))
    (`|SpawnActorFromClass` "/Game/Hank/Blueprints/Breakers_Open.Breakers_Open_C" (`self.breakertrans`) "Undefined" "OverrideRootScale")))

(event `Key|Five`
  (params (Key :type "Key Structure" :default "AnyKey"))
  (:`Pressed`
    (`/Game/Hank/Blueprints/Lightswitch.Event LightsDead` (`self.lightswitch`))
    (`/Game/Hank/Blueprints/Grandma.Event ScareOut` (`self.grandma`))))

(fn `UserConstructionScript`)