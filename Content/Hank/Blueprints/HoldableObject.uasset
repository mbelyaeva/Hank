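; HoldableObject is a flipbook-based prop that Hank can pick up and drop.
; On BeginPlay it caches the player pawn as Hank and builds a hidden highlight by duplicating its flipbook at a larger scale with an outline material.
; GrabbedByHank snaps the box collider to Hank's right-hand socket and disables physics and collision, while Dropped detaches it and restores both.
; The Selected event is empty, so nothing here reveals the highlight.
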(event `self.ReceiveBeginPlay`
  ;[1 1 1] Set reference to Hank
  (bind _ashank (cast `/Game/Hank/Blueprints/Hank` (`GameplayStatics.GetPlayerPawn` 0)))
  (set `self.hank` _ashank)
  ;[1 1 1] Add highlight effect
  (bind _returnvalue (`AddComponent|Paper Flipbook Component_0`))
  (bind _output_get (set `self.Highlight` _returnvalue))
  (`SceneComponent.SetRelativeScale3D` _output_get (* (`SceneComponent.RelativeScale3D` (`self.RenderComponent`)) (1.3 1.0 1.1)))
  (`PaperFlipbookComponent.SetFlipbook` (`self.Highlight`) (`PaperFlipbookComponent.GetFlipbook` (`self.RenderComponent`)))
  (`PrimitiveComponent.SetMaterial` (`self.Highlight`) 0 "/Game/Hank/Materials/Outline.Outline")
  (`SceneComponent.K2_SetRelativeLocation` (`self.Highlight`) (+ (`SceneComponent.RelativeLocation` (`self.Highlight`)) (0.0 -0.5 0.0)) false false)
  (`SceneComponent.SetVisibility` (`self.Highlight`) false false))

(event `Event GrabbedByHank`
  (`SceneComponent.K2_AttachTo` (`self.BoxCollider`) (`PaperCharacter.Sprite` (`self.Hank`)) "Right_Hand" "SnapToTarget" true)
  (`SceneComponent.K2_SetRelativeLocation` (`self.BoxCollider`) (20.0 0.0 0.0) false false)
  (`PrimitiveComponent.SetSimulatePhysics` (`self.BoxCollider`) false)
  (`PrimitiveComponent.SetCollisionEnabled` (`self.BoxCollider`) "NoCollision")
  (set `self.held` true))

(event `Event Dropped`
  (`SceneComponent.DetachFromParent` (`self.BoxCollider`) true true)
  (`PrimitiveComponent.SetCollisionEnabled` (`self.BoxCollider`) "QueryAndPhysics")
  (`PrimitiveComponent.SetSimulatePhysics` (`self.BoxCollider`) true)
  (set `self.held` false))

(event `Event Selected`)

(fn `UserConstructionScript`)