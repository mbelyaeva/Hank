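; Grandma is an NPC Blueprint that reacts to being scared, built on a parent class that also ticks.
; Scare drops the Duster, attaches a spawned flashlight to her right-hand socket and walks her toward the Lightswitch on a timer.
; Tick counts that timer down through Move, then turns the lights on and destroys the flashlight.
; ScareOut plays a scream and starts a much longer movement timer.
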(event `Event Move`
  (params (`Delta Seconds` :type "Float (double-precision)"))
  (if (`self.shouldMove`)
    (bind _output_get (set `self.moveTime` (- (`self.moveTime`) `Delta Seconds`)))
    (if (<= _output_get 0.0)
      (set `self.shouldMove` false)
      (`/Game/Hank/Blueprints/Lightswitch.Event LightsOn` (`self.lightswitch`))
      (`self.K2_DestroyActor` (stale `Event Scare` _returnvalue)))))

(event `Event Scare`
  (set `self.isScared` true)
  (`self.WalkToActor` (`self.lightswitch`))
  (bind _returnvalue (`|SpawnActorFromClass` "/Game/Hank/Blueprints/Flashlight_On.Flashlight_On_C" (`KismetMathLibrary.MakeTransform` (`SceneComponent.GetSocketLocation` (`self.RenderComponent`) "Right_Hand") (struct) (0.15 0.15 0.15)) "Undefined" "OverrideRootScale"))
  (`SceneComponent.K2_AttachTo` (`/Game/Hank/Blueprints/Flashlight_On.PaperSprite` _returnvalue) (`self.RenderComponent`) "Right_Hand" "KeepWorldPosition" true)
  (set `self.shouldMove` true)
  (set `self.moveDir` 1)
  (set `self.moveTime` 8.0)
  (`/Game/Hank/Blueprints/Duster.Event Dropped` (`self.duster`)))

(event `Event ScareOut`
  (set `self.shouldMove` true)
  (set `self.moveDir` 1)
  (set `self.moveTime` 1000.0)
  (`GameplayStatics.PlaySound2D` "/Game/Hank/Sounds/Female_Scream-SoundBible.Female_Scream-SoundBible" 1.0 1.0))

(event `self.ReceiveTick`
  (params (DeltaSeconds :type "Float (single-precision)"))
  (`self.Event Move` DeltaSeconds)
  (`parent.ReceiveTick` DeltaSeconds))

(fn `UserConstructionScript`)