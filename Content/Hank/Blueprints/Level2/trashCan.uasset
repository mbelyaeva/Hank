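; Interactable trash can Blueprint for Level 2 that shows a clown face on screen when the player interacts with it.
; On BeginPlay it calls the parent, creates a ClownFace widget and adds it to the viewport.
; The Interaction event calls ShowFace on that widget only when its face is not already visible.
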(event `self.ReceiveBeginPlay`
  (`parent.ReceiveBeginPlay`)
  (bind _returnvalue (`|CreateWidget` "/Game/Hank/Widgets/clownFace.clownFace_C"))
  (bind _output_get (set `self.widget` _returnvalue))
  (`UserWidget.AddToViewport` _output_get 0))

(event `self.Interaction`
  (params (heldItem :type "/Game/Hank/Blueprints/HoldableObject Object Reference"))
  (if (not (`/Game/Hank/Widgets/clownFace.faceVisible` (`self.widget`)))
    (`/Game/Hank/Widgets/clownFace.ShowFace` (`self.widget`))))

(fn `UserConstructionScript`
  (`parent.UserConstructionScript`))