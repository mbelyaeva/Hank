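; Interactable bunny prop in Level 2 that can be ripped open with scissors.
; Its Interaction event acts only when the held item is exactly of the Scissors class, then calls the parent interaction.
; It swaps the flipbook to the ripped bunny, spawns a Stuffing actor at its location and changes its description text.
; Nothing in this graph guards against repeat interactions.
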(event `self.Interaction`
  (params (heldItem :type "/Game/Hank/Blueprints/HoldableObject Object Reference"))
  (if (== (`GameplayStatics.GetObjectClass` heldItem) "/Game/Hank/Blueprints/Level2/scissors.scissors_C")
    (`parent.Interaction` heldItem)
    (`PaperFlipbookComponent.SetFlipbook` (`self.RenderComponent`) "/Game/Hank/Sprites/Level2/Objects/bunnyRipped_Flipbook.bunnyRipped_Flipbook")
    (`|SpawnActorFromClass` "/Game/Hank/Blueprints/Level2/stuffing.stuffing_C" (`KismetMathLibrary.MakeTransform` (`self.K2_GetActorLocation`)) "Undefined" "OverrideRootScale")
    (set `self.descriptionText` "Whoops.")))

(fn `UserConstructionScript`
  (`parent.UserConstructionScript`))