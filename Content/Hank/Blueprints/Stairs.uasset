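; Stairs actor that lets the player's Hank pawn move through it in Flying movement mode, acting as climbable stairs.
; BeginPlay caches player pawn 0 as Hank.
; Each Tick polls whether the RenderComponent overlaps Hank's capsule, switching his CharacterMovement to Flying while inside and back to Walking once outside.
; An IsFlying flag on the stairs limits mode changes to overlap transitions, without using overlap events.
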(event `self.ReceiveBeginPlay`
  (bind _ashank (cast `/Game/Hank/Blueprints/Hank` (`GameplayStatics.GetPlayerPawn` 0)))
  (set `self.hank` _ashank))

(event `self.ReceiveTick`
  (params (DeltaSeconds :type "Float (single-precision)"))
  (bind _charactermovement (`Character.CharacterMovement` (`self.hank`)))
  (if (`PrimitiveComponent.IsOverlappingComponent` (`self.RenderComponent`) (`Character.CapsuleComponent` (`self.hank`)))
    (if (not (`self.isFlying`))
      (`CharacterMovementComponent.SetMovementMode` _charactermovement "MOVE_Flying" 0)
      (set `self.isFlying` true))
    (elif (`self.isFlying`)
      (`CharacterMovementComponent.SetMovementMode` _charactermovement "MOVE_Walking" 0)
      (set `self.isFlying` false))))

(fn `UserConstructionScript`)