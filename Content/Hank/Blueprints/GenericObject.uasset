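; GenericObject is a Paper2D flipbook object that prepares a hidden outline highlight for itself.
; On BeginPlay it adds a second flipbook component that copies the render component's flipbook and uses the Outline material.
; The copy is scaled slightly larger and nudged along Y to form the outline, then left invisible.
; Nothing in this Blueprint shows the highlight; overlap, tick and construction logic are empty.
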(event `self.ReceiveBeginPlay`
  ;[1 1 1] Add highlight effect
  (bind _returnvalue (`AddComponent|PaperFlipbookComponent_1`))
  (bind _output_get (set `self.Highlight` _returnvalue))
  (`SceneComponent.SetRelativeScale3D` _output_get (* (`SceneComponent.RelativeScale3D` (`self.RenderComponent`)) (1.3 1.0 1.1)))
  (`PaperFlipbookComponent.SetFlipbook` (`self.Highlight`) (`PaperFlipbookComponent.GetFlipbook` (`self.RenderComponent`)))
  (`PrimitiveComponent.SetMaterial` (`self.Highlight`) 0 "/Game/Hank/Materials/Outline.Outline")
  (`SceneComponent.K2_SetRelativeLocation` (`self.Highlight`) (+ (`SceneComponent.RelativeLocation` (`self.Highlight`)) (0.0 -0.5 0.0)) false false)
  (`SceneComponent.SetVisibility` (`self.Highlight`) false false))

(event `self.ReceiveActorBeginOverlap`
  (params (OtherActor :type "Actor Object Reference")))

(event `self.ReceiveTick`
  (params (DeltaSeconds :type "Float (single-precision)")))

(fn `UserConstructionScript`)