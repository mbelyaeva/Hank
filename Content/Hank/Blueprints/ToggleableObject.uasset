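; ToggleableObject is a Blueprint for an object that flips between a primary and a secondary visual state.
; Toggle checks the Toggled flag and calls SwitchToPrimaryState or SwitchToSecondaryState, which can also be called directly to force a state.
; Each switch updates the flag and swaps visibility between RenderComponent and SecondarySprite, without propagating to child components.
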(event `self.ReceiveBeginPlay`
  (`parent.ReceiveBeginPlay`))

(event `Toggle`
  (if (`self.toggled`)
    (`self.SwitchToPrimaryState`)
    (else
      (`self.SwitchToSecondaryState`))))

(event `SwitchToPrimaryState`
  (set `self.toggled` false)
  (`SceneComponent.SetVisibility` (`self.RenderComponent`) true false)
  (`SceneComponent.SetVisibility` (`self.SecondarySprite`) false false))

(event `SwitchToSecondaryState`
  (set `self.toggled` true)
  (`SceneComponent.SetVisibility` (`self.RenderComponent`) false false)
  (`SceneComponent.SetVisibility` (`self.SecondarySprite`) true false))

(fn `UserConstructionScript`
  (`parent.UserConstructionScript`))