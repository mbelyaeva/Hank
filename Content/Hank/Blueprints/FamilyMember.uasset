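; Family member NPC on a Paper2D flipbook that walks queued routes and watches for Hank carrying objects.
; Tick moves it through queued horizontal or vertical steps, including fixed-height stair moves, and picks idle or walking animations with scared variants.
; Overlapping Hank while he holds something pauses walking, spawns question marks and steadily raises his suspicion.
; Direction toggles the left/right vision boxes and flips the sprite, refreshed on Tick only when the flipbook changes.
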(event Custom|Event%20PlayerEnterVision
  (Walking|PauseWalking)
  (bind _returnvalue (Game|SpawnActorfromClass "/Game/Hank/Blueprints/QuestionMarks.QuestionMarks_C" (Math|Transform|MakeTransform (+ (Transformation|GetWorldLocation (Variables|Default|GetBoxCollider)) "0, 0,130.000000") "0, 0, 0" "0.700000,0.700000,0.700000") "Undefined" 0 0)))

(event Custom|Event%20PlayerLeaveVision
  (Walking|ResumeWalking)
  (Actor|DestroyActor (stale Custom|Event%20PlayerEnterVision _returnvalue)))

(event EventBeginPlay
  (bind _ashank (Utilities|Casting|CastToHank (Game|Player|GetPlayerPawn 0)))
  (Variables|Default|Sethank _ashank)
  (Variables|Default|SetqueuedHeight (.Z (Math|Vector|BreakVector (Transformation|GetActorLocation)))))

(event Custom|Update%20Direction
  (bind _rendercomponent (Variables|Default|GetRenderComponent))
  (bind _rendercomponent_2 (Variables|Default|GetRenderComponent))
  (bind _visionright (Variables|Default|GetVisionRight))
  (bind _visionleft (Variables|Default|GetVisionLeft))
  (bind _rendercomponent_3 (Variables|Default|GetRenderComponent))
  (bind _relativescale3d (Variables|/Script/Engine.SceneComponent|GetRelativeScale3D _rendercomponent_3))
  (bind _relativescale3d_2 (Variables|/Script/Engine.SceneComponent|GetRelativeScale3D _rendercomponent_2))
  (bind (_x _y _z) (Math|Vector|BreakVector _relativescale3d))
  (bind (_x_2 _y_2 _z_2) (Math|Vector|BreakVector _relativescale3d_2))
  ;[1 1 1] Switch vision boxes based on direction
  (switch int (Variables|Default|Getdirection)
    (:0
      (Collision|SetCollisionEnabled _visionleft "QueryOnly")
      (Collision|SetCollisionEnabled _visionright "NoCollision")
      ;[1 1 1] Flip sprite when changing direction
      (Transformation|SetRelativeScale3D _rendercomponent (Math|Vector|MakeVector (* (Math|Float|Absolute(Float) _x) -1.0) _y _z)))
    (:1
      (Collision|SetCollisionEnabled _visionleft "NoCollision")
      (Collision|SetCollisionEnabled _visionright "NoCollision")
      (Transformation|SetRelativeScale3D _rendercomponent (Math|Vector|MakeVector (Math|Float|Absolute(Float) _x_2) _y_2 _z_2) :!label _label))
    (:2
      (Collision|SetCollisionEnabled _visionleft "NoCollision")
      (Collision|SetCollisionEnabled _visionright "QueryOnly")
      (goto _label))))

(event EventTick
  (params (DeltaSeconds :type Float%20%28single-precision%29))
  (bind _returnvalue (Transformation|GetActorLocation))
  (bind _returnvalue_2 (Transformation|GetActorLocation))
  (bind _self self)
  (bind _isscared (Variables|Default|GetisScared))
  (bind _rendercomponent (Variables|Default|GetRenderComponent))
  (bind _rendercomponent_2 (Variables|Default|GetRenderComponent))
  (bind _visionright (Variables|Default|GetVisionRight))
  (bind _visionleft (Variables|Default|GetVisionLeft))
  (bind _rendercomponent_3 (Variables|Default|GetRenderComponent))
  (bind _hank (Variables|Default|Gethank))
  (bind _movementqueue (Variables|Default|GetmovementQueue))
  (bind _movementqueue_2 (Variables|Default|GetmovementQueue))
  (bind _item (Utilities|Array|Get(acopy) _movementqueue))
  (bind _item_2 (Utilities|Array|Get(acopy) _movementqueue_2))
  (bind (_x _y _z) (Math|Vector|BreakVector _returnvalue))
  (bind (_x_2 _y_2 _z_2) (Math|Vector|BreakVector _returnvalue_2))
  (bind _relativescale3d (Variables|/Script/Engine.SceneComponent|GetRelativeScale3D _rendercomponent_3))
  (bind _relativescale3d_2 (Variables|/Script/Engine.SceneComponent|GetRelativeScale3D _rendercomponent_2))
  (bind _capsulecomponent (Variables|/Script/Engine.Character|GetCapsuleComponent _hank))
  (bind _holding (Variables|/Game/Hank/Blueprints/Hank.Hank_C|Getholding _hank))
  (bind _returnvalue_3 (Collision|IsOverlappingActor _capsulecomponent _self :!class /Script/Engine.PrimitiveComponent))
  (bind _z_3 (Math|Vector|BreakVector _item))
  (bind _x_3 (Math|Vector|BreakVector _item_2))
  (bind (_x_4 _y_3 _z_4) (Math|Vector|BreakVector _relativescale3d))
  (bind (_x_5 _y_4 _z_5) (Math|Vector|BreakVector _relativescale3d_2))
  (bind _returnvalue_4 (- _x_3 _x_2))
  (bind _returnvalue_5 (and _returnvalue_3 _holding))
  (bind _returnvalue_6 (> _returnvalue_4 0.0))
  (Variables|Default|SetdeltaSeconds DeltaSeconds)
  (if (and (not (Variables|Default|Getsuspicious)) _returnvalue_5) ; if not suspicious but should be
    (Variables|Default|Setsuspicious true)
    (CallFunction|EventPlayerEnterVision)
    (elif (and (Variables|Default|Getsuspicious) (not _returnvalue_5)) ; if suspicious but shouldn't be
      (Variables|Default|Setsuspicious false)
      (CallFunction|EventPlayerLeaveVision)))
  (if (Variables|Default|Getsuspicious)
    (Default|AddSuspicion (Variables|Default|Gethank) (* (Variables|Default|GetdeltaSeconds) 2e+01)))
  (if (and (Walking|HasWalkingTarget) (not (Variables|Default|GetwalkingPaused))) ; if need to move
    (if (Utilities|Array|Get(acopy) (Variables|Default|GetmovementQueue_vert))
      ;[1 1 1] Move towards target (vertical)
      (Transformation|SetActorLocation (Math|Vector|MakeVector _x _y (Math|Float|SelectFloat (Math|Float|Min(Float) _z_3 (+ _z (* (Variables|Default|GetdeltaSeconds) (Variables|Default|GetmoveSpeed)))) (Math|Float|Max(Float) _z_3 (- _z (* (Variables|Default|GetdeltaSeconds) (Variables|Default|GetmoveSpeed)))) (> (- _z_3 _z) 0.0))) false false)
      (if (!= _z_3 (.Z (Math|Vector|BreakVector (Transformation|GetActorLocation))))
        _
        (else
          (Utilities|Array|RemoveIndex (Variables|Default|GetmovementQueue))
          (Utilities|Array|RemoveIndex (Variables|Default|GetmovementQueue_vert))))
      (else
        ;[1 1 1] Move towards target (horizontal)
        (if _returnvalue_6
          (Variables|Default|Setdirection 2)
          (else
            (Variables|Default|Setdirection 0)))
        (Transformation|SetActorLocation (Math|Vector|MakeVector (Math|Float|SelectFloat (Math|Float|Min(Float) _x_3 (+ _x_2 (* (Variables|Default|GetdeltaSeconds) (Variables|Default|GetmoveSpeed)))) (Math|Float|Max(Float) _x_3 (- _x_2 (* (Variables|Default|GetdeltaSeconds) (Variables|Default|GetmoveSpeed)))) _returnvalue_6) _y_2 _z_2) false false)
        (if (!= _x_3 (.X (Math|Vector|BreakVector (Transformation|GetActorLocation))))
          _
          (else
            (Utilities|Array|RemoveIndex (Variables|Default|GetmovementQueue))
            (Utilities|Array|RemoveIndex (Variables|Default|GetmovementQueue_vert))))))
    ;[1 1 1] Switch between animations
    (if _isscared ; Walking Animations
      (Variables|Default|SetdesiredFlipbook (Variables|Animation|GetwalkingScaredAnim))
      (else
        (Variables|Default|SetdesiredFlipbook (Variables|Animation|GetwalkingAnim))))
    (else
      (if (Variables|Default|GetwalkingPaused)
        _
        (else
          (Variables|Default|Setdirection (Variables|Default|GetidleDirection))))
      (if _isscared ; Idle Animations
        (Variables|Default|SetdesiredFlipbook (Variables|Animation|GetidleScaredAnim))
        (else
          (Variables|Default|SetdesiredFlipbook (Variables|Animation|GetidleAnim))))))
  (if (not (== (Class|PaperFlipbookComponent|GetFlipbook (Variables|Default|GetRenderComponent)) (Variables|Default|GetdesiredFlipbook)))
    (Sprite|SetFlipbook (Variables|Default|GetRenderComponent) (Variables|Default|GetdesiredFlipbook))
    ;[1 1 1] Switch vision boxes based on direction
    (switch int (Variables|Default|Getdirection)
      (:0
        (Collision|SetCollisionEnabled _visionleft "QueryOnly")
        (Collision|SetCollisionEnabled _visionright "NoCollision")
        ;[1 1 1] Flip sprite when changing direction
        (Transformation|SetRelativeScale3D _rendercomponent (Math|Vector|MakeVector (* (Math|Float|Absolute(Float) _x_4) -1.0) _y_3 _z_4)))
      (:1
        (Collision|SetCollisionEnabled _visionleft "NoCollision")
        (Collision|SetCollisionEnabled _visionright "NoCollision")
        (Transformation|SetRelativeScale3D _rendercomponent (Math|Vector|MakeVector (Math|Float|Absolute(Float) _x_5) _y_4 _z_5) :!label _label))
      (:2
        (Collision|SetCollisionEnabled _visionleft "NoCollision")
        (Collision|SetCollisionEnabled _visionright "QueryOnly")
        (goto _label)))))

(fn ConstructionScript)

(fn WalktoActor
  (params (TargetActor :type Actor%20Object%20Reference) (Vertical :type Boolean))
  (Utilities|Array|Add (Variables|Default|GetmovementQueue) (Transformation|GetActorLocation TargetActor))
  (Utilities|Array|Add (Variables|Default|GetmovementQueue_vert) Vertical)
  (return))

(fn HasWalkingTarget
  (return (> (Utilities|Array|Length (Variables|Default|GetmovementQueue)) 0)))

(fn StopWalking
  (Utilities|Array|Clear (Variables|Default|GetmovementQueue))
  (Utilities|Array|Clear (Variables|Default|GetmovementQueue_vert))
  (Variables|Default|SetqueuedHeight (.Z (Math|Vector|BreakVector (Transformation|GetActorLocation))))
  (return))

(fn PauseWalking
  (Variables|Default|SetwalkingPaused true))

(fn ResumeWalking
  (Variables|Default|SetwalkingPaused false))

(fn WalkDownStairs
  (bind _output_get (Variables|Default|SetqueuedHeight (+ (Variables|Default|GetqueuedHeight) -3.5e+02)))
  (Utilities|Array|Add (Variables|Default|GetmovementQueue) (Math|Vector|MakeVector 0.0 0.0 _output_get))
  (Utilities|Array|Add (Variables|Default|GetmovementQueue_vert) (Class|KismetSystemLibrary|MakeLiteralBool true)))

(fn WalkUpStairs
  (bind _output_get (Variables|Default|SetqueuedHeight (+ (Variables|Default|GetqueuedHeight) 3.5e+02)))
  (Utilities|Array|Add (Variables|Default|GetmovementQueue) (Math|Vector|MakeVector 0.0 0.0 _output_get))
  (Utilities|Array|Add (Variables|Default|GetmovementQueue_vert) (Class|KismetSystemLibrary|MakeLiteralBool true)))