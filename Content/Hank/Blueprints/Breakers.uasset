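; Interactable breakers that act as the level exit trigger, killing the lights and scaring Grandma out before loading Level2.
; Interaction does nothing while either of two referenced web objects is still valid.
; Once clear, an untoggled interaction switches to the secondary state.
; A toggled one runs the parent interaction, fires events on Lightswitch and Grandma, then opens the next level after a short delay.
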(event `/Game/Hank/Blueprints/InteractableObject.Interaction`
  (params (heldItem :type "Actor Object Reference"))
  (if (or (`KismetSystemLibrary.IsValid` (`self.web1`)) (`KismetSystemLibrary.IsValid` (`self.web2`)))
    _
    (elif (`self.toggled`)
      (`parent.Interaction` heldItem)
      (`/Game/Hank/Blueprints/Lightswitch.Event LightsDead` (`self.lightswitch`))
      (`/Game/Hank/Blueprints/Grandma.Event ScareOut` (`self.grandma`))
      (`KismetSystemLibrary.Delay` 3.0)
      (`GameplayStatics.OpenLevel` "Level2")
      (else
        (`self.SwitchToSecondaryState`)))))

(fn `UserConstructionScript`)