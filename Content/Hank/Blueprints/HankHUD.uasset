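; HUD Blueprint for Hank that draws a suspicion meter, or a game-over page once Hank's GameOver flag is set.
; It caches the player pawn as Hank on BeginPlay and reads its state in each DrawHUD call.
; The meter layers a front texture over a fixed back, shifting and narrowing the front as Suspicion rises to uncover the back from the left.
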(event `self.ReceiveBeginPlay`
  (bind _ashank (cast `/Game/Hank/Blueprints/Hank` (`GameplayStatics.GetPlayerPawn` 0)))
  (set `self.hank` _ashank))

(event `self.ReceiveDrawHUD`
  (params (SizeX :type Integer) (SizeY :type Integer))
  (bind _suspicion (`/Game/Hank/Blueprints/Hank.suspicion` (`self.hank`)))
  (if (`/Game/Hank/Blueprints/Hank.gameOver` (`self.hank`))
    (`self.DrawTextureSimple` "/Game/Hank/Textures/Pages/Game_Over_Page.Game_Over_Page" 0.0 0.0 0.35)
    (else
      (`self.DrawTexture` "/Game/Hank/Textures/SuspicionMeter_back.SuspicionMeter_back" 10.0 10.0 400.0 50.0 0.0 0.0 1.0 1.0)
      (`self.DrawTexture` "/Game/Hank/Textures/SuspicionMeter_front.SuspicionMeter_front" (+ (* _suspicion 4.0) 10.0) 10.0 (- 400.0 (* _suspicion 4.0)) 50.0 0.0 0.0 1.0 1.0) ; TODO find nicer way to resize
    )))

(fn `UserConstructionScript`)