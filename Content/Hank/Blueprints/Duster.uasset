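; Duster is a Blueprint for a flipbook-rendered cleaning tool that Grandma holds and that clears webs.
; On BeginPlay it disables physics on its box collider, shows the still flipbook, attaches to Grandma's Right_Hand socket and marks itself held.
; On overlap it destroys any actor tagged Web, a handler flagged with a TODO fix.
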(event `self.ReceiveBeginPlay`
  (bind _boxcollider (`self.BoxCollider`))
  (`parent.ReceiveBeginPlay`)
  ;[1 1 1] Attach to Grandma
  (`PrimitiveComponent.SetSimulatePhysics` _boxcollider false)
  (`PaperFlipbookComponent.SetFlipbook` (`self.RenderComponent`) "/Game/Hank/Sprites/Level1/Objects/Duster_Still.Duster_Still")
  (`SceneComponent.K2_AttachTo` _boxcollider (`/Game/Hank/Blueprints/FamilyMember.RenderComponent` (`self.grandma`)) "Right_Hand" "KeepWorldPosition" true)
  (set `self.held` true))

(event `self.ReceiveActorBeginOverlap`
  (params (OtherActor :type "Actor Object Reference"))
  ;[1 1 1] TODO fix
  (if (`self.ActorHasTag` OtherActor "Web")
    (`self.K2_DestroyActor` OtherActor)))

(fn `UserConstructionScript`)